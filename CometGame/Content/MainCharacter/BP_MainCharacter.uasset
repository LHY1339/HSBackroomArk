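; Player character that handles movement, look, jump and run/walk speed input, and tracks motion values.
; Input events pass through handlers gated by a per-action permission map (Full, Limit, Ban), of which only Full is acted on.
; Each tick, the locally controlled instance calculates speed, direction and view-angle offsets, then sends them through a server update event.
; GetVariable exposes these values, and SetMoveMotion edits existing permissions.
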(event EventTick
  (params (DeltaSeconds :type Float%20%28single-precision%29))
  (Utilities|FlowControl|Sequence
    (:then_0
      (if (Pawn|IsLocallyControlled)
        (Utilities|FlowControl|Sequence
          (:then_0
            (private|CalculateVaribale))
          (:then_1
            (CallFunction|UpdateVaribaleServer (Variables|Replicated|GetSpeedXY) (Variables|Replicated|GetSpeedZ) (Variables|Replicated|GetDirection) (Variables|Replicated|GetPitch) (Variables|Replicated|GetYaw))))))))

(event EventBeginPlay)

(event Input|ActionEvents|InputActionJump
  (params (Key :type Key%20Structure))
  (:Pressed
    (CallFunction|ActionJump "NewEnumerator0"))
  (:Released
    (CallFunction|ActionJump "NewEnumerator1")))

(event Input|ActionEvents|InputActionRun
  (params (Key :type Key%20Structure))
  (:Pressed
    (CallFunction|ActionRun "NewEnumerator0"))
  (:Released
    (CallFunction|ActionRun "NewEnumerator1")))

(event Input|ActionEvents|InputActionWalk
  (params (Key :type Key%20Structure))
  (:Pressed
    (CallFunction|ActionWalk "NewEnumerator0"))
  (:Released
    (CallFunction|ActionWalk "NewEnumerator1")))

(event Input|AxisEvents|InputAxisMoveForward
  (params (AxisValue :type Float%20%28single-precision%29))
  (CallFunction|AxisMoveForward AxisValue))

(event Input|AxisEvents|InputAxisMoveRight
  (params (AxisValue :type Float%20%28single-precision%29))
  (CallFunction|AxisMoveRight AxisValue))

(event Input|AxisEvents|InputAxisLookUp
  (params (AxisValue :type Float%20%28single-precision%29))
  (CallFunction|AxisLookUp AxisValue))

(event Input|AxisEvents|InputAxisLookRight
  (params (AxisValue :type Float%20%28single-precision%29))
  (CallFunction|AxisLookRight AxisValue))

(event Custom|Axis_LookRight
  (params (Value :type Float%20%28single-precision%29))
  (Utilities|GetMoveMotion "LookRight"
    (:Full
      (Pawn|Input|AddControllerYawInput Value))))

(event Custom|Axis_LookUp
  (params (Value :type Float%20%28single-precision%29))
  (Utilities|GetMoveMotion "LookUp"
    (:Full
      (Pawn|Input|AddControllerPitchInput Value))))

(event Custom|Action_Jump
  (params (Input :type EInputMotion%20Enum :default "NewEnumerator0"))
  (bind _output_get (Variables|Private|Setvar_IsJump Input))
  (switch Utilities|FlowControl|Switch|SwitchonEInputMotion _output_get
    (:NewEnumerator0
      (Utilities|GetMoveMotion "Jump"
        (:Full
          (Character|Jump))))
    (:NewEnumerator1
      (Character|StopJumping))))

(event Custom|Axis_MoveRight
  (params (Value :type Float%20%28single-precision%29))
  (Utilities|GetMoveMotion "MoveRight"
    (:Full
      (Pawn|Input|AddMovementInput (Math|Vector|GetRightVector (Math|Rotator|MakeRotator 0.0 0.0 (.yaw (Pawn|GetControlRotation :!class /Script/Engine.Pawn)))) Value false))))

(event Custom|Axis_MoveForward
  (params (Value :type Float%20%28single-precision%29))
  (Utilities|GetMoveMotion "MoveForward"
    (:Full
      (Pawn|Input|AddMovementInput (Math|Vector|GetForwardVector (Math|Rotator|MakeRotator 0.0 0.0 (.yaw (Pawn|GetControlRotation :!class /Script/Engine.Pawn)))) Value false))))

(event Custom|Action_Run
  (params (Input :type EInputMotion%20Enum :default "NewEnumerator0"))
  (bind _output_get (Variables|Private|Setvar_IsRun Input))
  (switch Utilities|FlowControl|Switch|SwitchonEInputMotion _output_get
    (:NewEnumerator0
      (Utilities|GetMoveMotion "Run"
        (:Full
          (Class|HSCharacter|SetMaxWalkSpeed 6e+02))))
    (:NewEnumerator1
      (switch Utilities|FlowControl|Switch|SwitchonEInputMotion (Variables|Private|Getvar_IsWalk)
        (:NewEnumerator0
          (Class|HSCharacter|SetMaxWalkSpeed 1e+02))
        (:NewEnumerator1
          (Class|HSCharacter|SetMaxWalkSpeed 4e+02))))))

(event Custom|Action_Walk
  (params (Input :type EInputMotion%20Enum :default "NewEnumerator0"))
  (bind _output_get (Variables|Private|Setvar_IsWalk Input))
  (switch Utilities|FlowControl|Switch|SwitchonEInputMotion _output_get
    (:NewEnumerator0
      (Utilities|GetMoveMotion "Walk"
        (:Full
          (switch Utilities|FlowControl|Switch|SwitchonEInputMotion (Variables|Private|Getvar_IsRun)
            (:NewEnumerator1
              (Class|HSCharacter|SetMaxWalkSpeed 1e+02))))))
    (:NewEnumerator1
      (switch Utilities|FlowControl|Switch|SwitchonEInputMotion (Variables|Private|Getvar_IsRun)
        (:NewEnumerator1
          (Class|HSCharacter|SetMaxWalkSpeed 4e+02))))))

(event Custom|UpdateVaribale_Server
  (params (SpeedXY :type Float%20%28single-precision%29) (SpeedZ :type Float%20%28single-precision%29) (Direction :type Float%20%28single-precision%29) (Pitch :type Float%20%28single-precision%29) (Yaw :type Float%20%28single-precision%29))
  (Variables|Replicated|SetSpeedXY SpeedXY)
  (Variables|Replicated|SetSpeedZ SpeedZ)
  (Variables|Replicated|SetDirection Direction)
  (Variables|Replicated|SetPitch Pitch)
  (Variables|Replicated|SetYaw Yaw))

(fn ConstructionScript)

(fn CalculateVaribale
  (Utilities|FlowControl|Sequence
    (:then_0
      (Utilities|FlowControl|Sequence
        (:then_0
          (|cal_speed))
        (:then_1
          (|cal_direction))
        (:then_2
          (|cal_viewangle))))
    (:then_1
      (return))))

(fn GetVariable
  (return (Variables|Replicated|GetSpeedXY) (Variables|Replicated|GetSpeedZ) (Variables|Replicated|GetDirection) (Variables|Replicated|GetPitch) (Variables|Replicated|GetYaw)))

(fn GetCharacter
  (return self))